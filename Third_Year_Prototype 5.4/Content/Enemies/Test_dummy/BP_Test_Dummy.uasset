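; BP_Test_Dummy is a test enemy with a zombie melee attack, HP and a proximity health bar.
; Attack stops movement and plays a montage, immediately sphere-checking for the player character to subtract HP, with walking restored shortly after completion.
; The attack lock clears after a delay only on a hit, so a miss leaves it set.
; The Range overlap toggles the health bar, and Tick destroys the actor at exactly zero HP.
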(event OnComponentBeginOverlap(Range)
  (params (OverlappedComponent :type Primitive%20Component%20Object%20Reference) (OtherActor :type Actor%20Object%20Reference) (OtherComp :type Primitive%20Component%20Object%20Reference) (OtherBodyIndex :type Integer) (bFromSweep :type Boolean) (SweepResult :type Hit%20Result%20Structure%20%28by%20ref%29))
  (Rendering|SetVisibility (Variables|Default|GetHealth%20Bar) true false))

(event OnComponentEndOverlap(Range)
  (params (OverlappedComponent :type Primitive%20Component%20Object%20Reference) (OtherActor :type Actor%20Object%20Reference) (OtherComp :type Primitive%20Component%20Object%20Reference) (OtherBodyIndex :type Integer))
  (Rendering|SetVisibility (Variables|Default|GetHealth%20Bar) false false))

(event Custom|Attack
  (if (not (Variables|Default|GetIs%20Attacking?))
    (Variables|Default|SetIs%20Attacking? true)
    (Pawn|Components|CharacterMovement|DisableMovement (Variables|Character|GetCharacterMovement))
    (Animation|Montage|PlayMontage (Variables|Character|GetMesh) "/Game/BSP_ZombieAnims/Animations/Standing/Attack/AM_ZombieAttack.AM_ZombieAttack"
      (:then
        (bind _outactors (Collision|SphereOverlapActors (Transformation|GetWorldLocation (Variables|Default|GetSphere%20attack)) 1e+02 (Utilities|Array|MakeArray "ObjectTypeQuery3") "/Game/ThirdPerson/Blueprints/BP_ThirdPersonCharacter.BP_ThirdPersonCharacter_C" (Utilities|Array|MakeArray self)))
        (if (Utilities|Array|IsValidIndex _outactors)
          (bind _asbp_third_person_character (Utilities|Casting|CastToBP_ThirdPersonCharacter (Game|GetPlayerCharacter 0)))
          (Variables|/Game/ThirdPerson/Blueprints/BP_ThirdPersonCharacter.BP_ThirdPersonCharacter_C|SetCurrent%20HP _asbp_third_person_character (- (Variables|/Game/ThirdPerson/Blueprints/BP_ThirdPersonCharacter.BP_ThirdPersonCharacter_C|GetCurrent%20HP _asbp_third_person_character) 1e+01))
          (Utilities|FlowControl|Delay 3.0)
          (Variables|Default|SetIs%20Attacking? false)))
      (:OnCompleted
        (Utilities|FlowControl|Delay 1.0)
        (Pawn|Components|CharacterMovement|SetMovementMode (Variables|Character|GetCharacterMovement) "MOVE_Walking" 0)))))

(event EventTick
  (params (DeltaSeconds :type Float%20%28single-precision%29))
  (if (== (Variables|Default|GetHP) 0.0)
    (Actor|DestroyActor)))

(fn ConstructionScript)